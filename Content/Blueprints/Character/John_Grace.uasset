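; John_Grace is the player character, with montage-driven melee, blocking, camera-relative movement and a launch-based dash with cooldown.
; Attacking and Blocking flags gate each other and weapon swapping, which cycles the attack montage but always respawns a hand-attached Bread_Sword.
; Damage updates Health and the HUD, setting a Dead flag that Tick polls to pause and show the death screen.
; It also holds music, pause menu, broken save/load and debug keys.
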(event Custom|BattleMusic
  (bind _returnvalue (Audio|SpawnSound2D 0 1.0 1.0 0.0 0))
  (Variables|Default|SetCombat%20music _returnvalue))

(event Custom|Save%20Game
  ;[0.1406 0.008057 0.008057 0.5] Game Save [BROKEN]
  (bind _returnvalue (SaveGame|CreateSaveGameObject "/Game/Blueprints/Character/Support/Save+Load.Save+Load_C"))
  (Variables|/Game/Blueprints/Character/Support/Save+Load.Save+Load_C|SetPlayerHealth _returnvalue (Variables|Default|GetHealth))
  (SaveGame|SaveGametoSlot _returnvalue "1"))

(event Custom|Load%20Game
  ;[0.1406 0.008057 0.008057 0.5] Game Save [BROKEN]
  (SaveGame|CreateSaveGameObject "/Game/Blueprints/Character/Support/Save+Load.Save+Load_C")
  (SaveGame|LoadGamefromSlot "1"))

(event Custom|Activate%20HUD
  (bind _returnvalue (UserInterface|CreateWidget "/Game/Blueprints/Character/Widgets/JG_HUD.JG_HUD_C" (Game|GetPlayerController 0)))
  (UserInterface|Viewport|AddtoPlayerScreen _returnvalue))

(event Input|EnhancedActionEvents|EnhancedInputActionIA_Dash
  (params (ActionValue :type Boolean) (ElapsedSeconds :type Float%20%28double-precision%29) (TriggeredSeconds :type Float%20%28double-precision%29) (InputAction :type Input%20Action%20Object%20Reference :default "/Game/Blueprints/Character/Input_Maps/Input_Act/IA_Dash.IA_Dash"))
  ;[0.3116 0.8438 0.07031 0.5] Movement
  (Pawn|Components|CharacterMovement|SetMovementMode (Variables|Character|GetCharacterMovement) "MOVE_Walking" 0)
  (if (|MovementCheck)
    (if (not (Variables|Default|GetIn%20cooldown))
      (CallFunction|Dash)
      (Variables|Default|SetIn%20cooldown true)
      (Animation|Montage|PlayMontage (Variables|Character|GetMesh) "/Game/Animation/MM_Death_Back_01_Montage.MM_Death_Back_01_Montage"
        (:then
          (Variables|Default|SetAttacking false)
          (Utilities|FlowControl|Delay 1.0)
          (Variables|Default|SetIn%20cooldown false))))))

(event Input|EnhancedActionEvents|EnhancedInputActionIA_Meele
  (params (ActionValue :type Boolean) (ElapsedSeconds :type Float%20%28double-precision%29) (TriggeredSeconds :type Float%20%28double-precision%29) (InputAction :type Input%20Action%20Object%20Reference :default "/Game/Blueprints/Character/Input_Maps/Input_Act/IA_Meele.IA_Meele"))
  (:Started
    (if (not (Variables|Default|GetBlocking))
      (Pawn|Components|CharacterMovement|SetMovementMode (Variables|Character|GetCharacterMovement) "MOVE_None" 0)
      (Variables|Default|SetAttacking true)
      (switch Utilities|FlowControl|Switch|SwitchonE_CurrentWeapon (Variables|Default|GetCurrent%20Weapon%20num)
        (:NewEnumerator0
          (Animation|Montage|PlayMontage (Variables|Character|GetMesh) "/Game/Blueprints/Enemies/Enemy_Animation/Montage_attack.Montage_attack"
            (:OnCompleted
              (Pawn|Components|CharacterMovement|SetMovementMode (Variables|Character|GetCharacterMovement) "MOVE_Walking" 0)
              (Variables|Default|SetAttacking false))))
        (:NewEnumerator1
          (Animation|Montage|PlayMontage (Variables|Character|GetMesh) "/Game/Blueprints/Enemies/Enemy_Animation/AS_SpellAttack_Montage.AS_SpellAttack_Montage"
            (:OnCompleted
              (Pawn|Components|CharacterMovement|SetMovementMode (Variables|Character|GetCharacterMovement) "MOVE_Walking" 0)
              (Variables|Default|SetAttacking false))))
        (:NewEnumerator2
          (Animation|Montage|PlayMontage (Variables|Character|GetMesh) "/Game/Animation/MM_Death_Back_01_Montage.MM_Death_Back_01_Montage"
            (:OnCompleted
              (Pawn|Components|CharacterMovement|SetMovementMode (Variables|Character|GetCharacterMovement) "MOVE_Walking" 0)
              (Variables|Default|SetAttacking false))))))))

(event Input|EnhancedActionEvents|EnhancedInputActionIA_Move
  (params (ActionValue :type Vector%202D%20Structure) (ElapsedSeconds :type Float%20%28double-precision%29) (TriggeredSeconds :type Float%20%28double-precision%29) (InputAction :type Input%20Action%20Object%20Reference :default "/Game/Blueprints/Character/Input_Maps/Input_Act/IA_Move.IA_Move"))
  ;[0.3116 0.8438 0.07031 0.5] Movement
  (CallFunction|Move (.x ActionValue) (.y ActionValue)))

(event Input|EnhancedActionEvents|EnhancedInputActionIA_Parry-Block
  (params (ActionValue :type Boolean) (ElapsedSeconds :type Float%20%28double-precision%29) (TriggeredSeconds :type Float%20%28double-precision%29) (InputAction :type Input%20Action%20Object%20Reference :default "/Game/Blueprints/Character/Input_Maps/Input_Act/IA_Parry-Block.IA_Parry-Block"))
  (:Triggered
    (if (not (Variables|Default|GetAttacking))
      (Variables|Default|SetBlocking true)
      (Pawn|Components|CharacterMovement|SetMovementMode (Variables|Character|GetCharacterMovement) "MOVE_None" 0)
      (Animation|Montage|PlayMontage (Variables|Character|GetMesh) "/Game/Blueprints/Enemies/Enemy_Animation/Montage_attack.Montage_attack")))
  (:Completed
    (Variables|Default|SetBlocking false)
    (Animation|StopAnimMontage "/Game/Blueprints/Enemies/Enemy_Animation/Montage_attack.Montage_attack")
    (Pawn|Components|CharacterMovement|SetMovementMode (Variables|Character|GetCharacterMovement) "MOVE_Walking" 0)))

(event EventTick
  (params (DeltaSeconds :type Float%20%28single-precision%29))
  (if (Variables|Default|GetDead)
    (CallFunction|Death)))

(event Game|Damage|EventAnyDamage
  (params (Damage :type Float%20%28single-precision%29) (DamageType :type Damage%20Type%20Object%20Reference) (InstigatedBy :type Controller%20Object%20Reference) (DamageCauser :type Actor%20Object%20Reference))
  ;[0.06956 1 0.05217 0.5] Damage Control
  (Variables|Default|SetHealth (- (Variables|Default|GetHealth) Damage))
  (Default|HealthUpdate (Variables|Default|GetHUD%20Ref))
  (if (<= (Variables|Default|GetHealth) 0.0)
    (Variables|Default|SetDead true)))

(event EventBeginPlay
  (Variables|Default|SetHealth (Variables|Default|GetMaxHealth))
  (bind _asgi_audio_manager (Utilities|Casting|CastToGI_AudioManager (Game|GetGameInstance)))
  (Default|PlayBackgroundMusic _asgi_audio_manager)
  (bind _returnvalue (Game|SpawnActorfromClass "/Game/Blueprints/Character/Weapons/Bread_Sword.Bread_Sword_C" (Transformation|GetActorTransform) "Undefined" "MultiplyWithRoot" 0 0))
  (bind _output_get (Variables|Default|SetCurrent%20Weapon _returnvalue))
  (Transformation|AttachComponentToComponent _output_get (Variables|Character|GetMesh) "HandGrip_R" "SnapToTarget" "SnapToTarget" "SnapToTarget" true))

(event Input|KeyboardEvents|1
  (params (Key :type Key%20Structure :default "None"))
  ;[0.6073 0.5288 0.02594 0.5] TEST
  (:Pressed
    (bind _returnvalue (Actor|GetActorOfClass "/Game/Blueprints/Enemies/BP_EnemyParent.BP_EnemyParent_C"))
    (bind _asaic_enemy_parent (Utilities|Casting|CastToAIC_EnemyParent (AI|GetAIController _returnvalue)))
    (Utilities|FlowControl|FlipFlop
      (:A
        (Default|SetStateasAttacking _asaic_enemy_parent self))
      (:B
        (Default|SetStateasPassive _asaic_enemy_parent)))))

(event Input|KeyboardEvents|2
  (params (Key :type Key%20Structure :default "None"))
  ;[0.6073 0.5288 0.02594 0.5] TEST
  (:Pressed
    (Game|Damage|ApplyDamage self (Variables|Default|GetDamagetest) 0 0)))

(event Input|KeyboardEvents|F
  (params (Key :type Key%20Structure :default "None"))
  (:Pressed
    (CallFunction|WeaponSwap)))

(event Input|KeyboardEvents|F
  (params (Key :type Key%20Structure :default "None"))
  ;[0.6073 0.5288 0.02594 0.5] TEST
  (:Pressed
    (bind _returnvalue (Actor|GetActorOfClass "/Game/Blueprints/Enemies/BP_EnemyParent.BP_EnemyParent_C"))
    (Class|AISenseDamage|ReportDamageEvent _returnvalue self 2e+01 (Transformation|GetActorLocation) "0, 0, 0" "None")))

(event Input|KeyboardEvents|Escape
  (params (Key :type Key%20Structure :default "None"))
  (:Pressed
    (bind _returnvalue (UserInterface|CreateWidget "/Game/Blueprints/Character/Widgets/Pause_Menu.Pause_Menu_C"))
    (UserInterface|Viewport|AddtoPlayerScreen _returnvalue)))

(fn ConstructionScript)

(fn Move
  (params (Left%20/%20Right :type Float%20%28double-precision%29) (Forward%20/%20Backward :type Float%20%28double-precision%29))
  (bind _returnvalue (Pawn|GetControlRotation :!class /Script/Engine.Pawn))
  ;[0.15 0.15 0.15 0.5] L/R
  (Pawn|Input|AddMovementInput (Math|Vector|GetRightVector (Math|Rotator|MakeRotator 0.0 0.0 (.yaw _returnvalue))) Left%20/%20Right false)
  ;[0.15 0.15 0.15 0.5] F/B
  (Pawn|Input|AddMovementInput (Math|Vector|GetForwardVector (Math|Rotator|MakeRotator 0.0 0.0 (.yaw _returnvalue))) Forward%20/%20Backward false))

(fn Dash
  (Character|LaunchCharacter (* (Pawn|Components|PawnMovement|GetLastInputVector (Variables|Character|GetCharacterMovement)) 2.5e+03) false false))

(fn Death
  (Game|SetGamePaused true)
  (bind _returnvalue (UserInterface|CreateWidget "/Game/Blueprints/Character/Widgets/JG_Death.JG_Death_C"))
  (UserInterface|Viewport|AddtoViewport _returnvalue 0))

(fn WeaponSwap
  (if (not (or (Variables|Default|GetAttacking) (Variables|Default|GetBlocking)))
    (switch Utilities|FlowControl|Switch|SwitchonE_CurrentWeapon (Variables|Default|GetCurrent%20Weapon%20num)
      (:NewEnumerator0
        (Actor|DestroyActor (Variables|Default|GetCurrent%20Weapon))
        (bind _returnvalue (Game|SpawnActorfromClass "/Game/Blueprints/Character/Weapons/Bread_Sword.Bread_Sword_C" (Transformation|GetActorTransform) "Undefined" "MultiplyWithRoot" 0 0))
        (bind _output_get (Variables|Default|SetCurrent%20Weapon _returnvalue))
        (Transformation|AttachComponentToComponent _output_get (Variables|Character|GetMesh) "HandGrip_R" "SnapToTarget" "SnapToTarget" "SnapToTarget" true)
        (Variables|Default|SetCurrent%20Weapon%20num "NewEnumerator1"))
      (:NewEnumerator1
        (Actor|DestroyActor (Variables|Default|GetCurrent%20Weapon))
        (bind _returnvalue_2 (Game|SpawnActorfromClass "/Game/Blueprints/Character/Weapons/Bread_Sword.Bread_Sword_C" (Transformation|GetActorTransform) "Undefined" "MultiplyWithRoot" 0 0))
        (bind _output_get_2 (Variables|Default|SetCurrent%20Weapon _returnvalue_2))
        (Transformation|AttachComponentToComponent _output_get_2 (Variables|Character|GetMesh) "HandGrip_R" "SnapToTarget" "SnapToTarget" "SnapToTarget" true)
        (Variables|Default|SetCurrent%20Weapon%20num "NewEnumerator2"))
      (:NewEnumerator2
        (Actor|DestroyActor (Variables|Default|GetCurrent%20Weapon))
        (bind _returnvalue_3 (Game|SpawnActorfromClass "/Game/Blueprints/Character/Weapons/Bread_Sword.Bread_Sword_C" (Transformation|GetActorTransform) "Undefined" "MultiplyWithRoot" 0 0))
        (bind _output_get_3 (Variables|Default|SetCurrent%20Weapon _returnvalue_3))
        (Transformation|AttachComponentToComponent _output_get_3 (Variables|Character|GetMesh) "HandGrip_R" "SnapToTarget" "SnapToTarget" "SnapToTarget" true)
        (Variables|Default|SetCurrent%20Weapon%20num "NewEnumerator0")))))