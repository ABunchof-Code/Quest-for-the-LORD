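; BP_patrol_route is a spline-based patrol route for enemy AI that tracks a current point along the path.
; IncrementPatrolRoute steps the index by the current direction and flips that direction at the first and last spline points, producing a back-and-forth patrol.
; GetSplinePointAsWorldPostion returns the world location of the current spline point.
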(event Custom|IncrementPatrolRoute
  (bind _output_get (Variables|Default|SetIndex (+ (Variables|Default|GetIndex) (Variables|Default|GetDirection))))
  (if (== _output_get (- (Spline|GetNumberOfSplinePoints (Variables|Default|GetPatrol%20route)) 1))
    (Variables|Default|SetDirection -1)
    (elif (== (Variables|Default|GetIndex) 0)
      (Variables|Default|SetDirection 1))))

(fn ConstructionScript)

(fn GetSplinePointasWorldPostion
  (return (Spline|GetLocationatSplinePoint (Variables|Default|GetPatrol%20route) (Variables|Default|GetIndex) "World")))