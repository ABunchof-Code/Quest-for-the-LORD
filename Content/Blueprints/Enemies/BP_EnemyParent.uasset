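; Base enemy character that carries a sword, takes damage and supplies attacks, patrol route and walk/run speeds.
; BeginPlay sets starting health and attaches a spawned sword to the hand socket.
; Two montage attacks fire an attack-end dispatcher when completed or interrupted, and combat music starts once and fades out on stop.
; Damage checks health before subtracting, so a hit after health is depleted destroys sword and enemy.
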(event Custom|HoldSword
  (bind _returnvalue (Game|SpawnActorfromClass "/Game/Blueprints/Enemies/Enemy_Weapon/BP_ESword.BP_ESword_C" (Transformation|GetActorTransform) "Undefined" "MultiplyWithRoot" 0 0))
  (bind _output_get (Variables|Default|SetSword _returnvalue))
  (Transformation|AttachComponentToComponent _output_get (Variables|Character|GetMesh) "hand_r_wep" "SnapToTarget" "SnapToTarget" "SnapToTarget" true))

(event Custom|Attack
  (Animation|Montage|PlayMontage (Variables|Character|GetMesh) "/Game/Blueprints/Enemies/Enemy_Animation/Montage_attack.Montage_attack"
    (:OnCompleted
      _)
    (:OnInterrupted
      _))
  (Default|CallOnAttackEnd))

(event Custom|Attack2
  (Animation|Montage|PlayMontage (Variables|Character|GetMesh) "/Game/Blueprints/Enemies/Enemy_Animation/AS_SpellAttack_Montage.AS_SpellAttack_Montage"
    (:OnCompleted
      _)
    (:OnInterrupted
      _))
  (Default|CallOnAttackEnd))

(event Custom|PlayMusic
  (if (not (Variables|Default|GetIsMusicPlaying))
    (Variables|Default|SetIsMusicPlaying true)
    (bind _returnvalue (Audio|SpawnSound2D 0 1.0 1.0 0.0 0))
    (Variables|Default|SetCombatMusic _returnvalue)))

(event Custom|StopMusic
  (bind _combatmusic (Variables|Default|GetCombatMusic)
    (:then
      (Audio|Components|Audio|FadeOut _combatmusic 2.0 0.0 "Linear" :!class /Script/Engine.AudioComponent)
      (Variables|Default|SetIsMusicPlaying false))
    (:else)))

(event EventBeginPlay
  (CallFunction|HoldSword)
  (Variables|Default|Sethealth (Variables|Default|GetM-Health)))

(event Game|Damage|EventAnyDamage
  (params (Damage :type Float%20%28single-precision%29) (DamageType :type Damage%20Type%20Object%20Reference) (InstigatedBy :type Controller%20Object%20Reference) (DamageCauser :type Actor%20Object%20Reference))
  (if (> (Variables|Default|Gethealth) 0)
    (Development|PrintString "i am not dead")
    (Variables|Default|Sethealth (- (Variables|Default|Gethealth) Damage))
    (else
      (Development|PrintString "I am dead")
      (Actor|DestroyActor (Variables|Default|GetSword))
      (Actor|DestroyActor))))

(fn ConstructionScript)

(fn GetPatrolRoute
  (return (Variables|Default|GetPatrolRoute)))

(fn SetMovementSpeed
  (params (Speed :type E_MovementSpeed%20Enum :default "NewEnumerator0"))
  (bind _output_get (Variables|/Script/Engine.CharacterMovementComponent|SetMaxWalkSpeed (Variables|Character|GetCharacterMovement) (Utilities|Select :Index Speed :NewEnumerator0 1.5e+02 :NewEnumerator1 3e+02)))
  (return _output_get))