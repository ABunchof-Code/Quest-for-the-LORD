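; Boss enemy Blueprint that provides two attack events, Attack and Attack2.
; Each sets the Attacking flag and plays the boss montage on the mesh, then clears the flag and calls the OnAttackEnd dispatcher on completion or interruption.
; Both events are currently identical, using the same montage, and the file adds no BeginPlay or construction logic of its own.
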(event EventBeginPlay
  (|CallParentFunction) ; This node is disabled and will not be called.\nDrag off pins to build functionality.
)

(event EventAttack
  (Variables|Default|SetAttacking true)
  (Animation|Montage|PlayMontage (Variables|Character|GetMesh) "/Game/Blueprints/Enemies/Enemy_Animation/boss_Anim_Montage.boss_Anim_Montage"
    (:OnCompleted
      _)
    (:OnInterrupted
      _))
  (Variables|Default|SetAttacking false)
  (Default|CallOnAttackEnd))

(event EventAttack2
  (Variables|Default|SetAttacking true)
  (Animation|Montage|PlayMontage (Variables|Character|GetMesh) "/Game/Blueprints/Enemies/Enemy_Animation/boss_Anim_Montage.boss_Anim_Montage"
    (:OnCompleted
      _)
    (:OnInterrupted
      _))
  (Variables|Default|SetAttacking false)
  (Default|CallOnAttackEnd))

(fn ConstructionScript
  (|CallParentFunction))