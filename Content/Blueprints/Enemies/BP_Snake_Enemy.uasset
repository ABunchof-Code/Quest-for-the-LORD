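; Snake enemy Blueprint that provides two attacks, a standard one and a ranged one, each setting damage and an attacking flag before playing its montage.
; The standard attack's montage notifies switch Hurtbox collision on and off, and Hurtbox overlaps apply the current damage.
; The ranged attack only plays its montage here, with no projectile or hitbox logic.
; Both attacks clear the flag and fire OnAttackEnd on completion or interruption.
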(event OnComponentBeginOverlap(Hurtbox)
  (params (OverlappedComponent :type Primitive%20Component%20Object%20Reference) (OtherActor :type Actor%20Object%20Reference) (OtherComp :type Primitive%20Component%20Object%20Reference) (OtherBodyIndex :type Integer) (bFromSweep :type Boolean) (SweepResult :type Hit%20Result%20Structure%20%28by%20ref%29))
  (Game|Damage|ApplyDamage 0 (Math|Conversions|ToFloat(Integer) (Variables|Default|Getdamage)) 0 0))

(event EventBeginPlay
  (|CallParentFunction) ; This node is disabled and will not be called.\nDrag off pins to build functionality.
)

(event EventAttack
  (Variables|Default|Setdamage 3)
  (Variables|Default|SetAttacking true)
  (bind _notifyname (Animation|Montage|PlayMontage (Variables|Character|GetMesh) "/Game/Blueprints/Enemies/Enemy_Animation/Snake_attack_Anim_Montage.Snake_attack_Anim_Montage")
    (:OnCompleted
      (Variables|Default|SetAttacking false :!label _label)
      (Default|CallOnAttackEnd))
    (:OnInterrupted
      (goto _label))
    (:OnNotifyBegin
      (switch name _notifyname
        (:attack%20begin
          (Collision|SetCollisionProfileName (Variables|Default|GetHurtbox) "OverlapAllDynamic" true :!class /Script/Engine.PrimitiveComponent))
        (:attack%20end
          (Collision|SetCollisionProfileName (Variables|Default|GetHurtbox) "NoCollision" true :!class /Script/Engine.PrimitiveComponent))))))

(event EventAttack2
  (Variables|Default|Setdamage 5)
  (Variables|Default|SetAttacking true)
  (Animation|Montage|PlayMontage (Variables|Character|GetMesh) "/Game/Blueprints/Enemies/Enemy_Animation/Snake_range_attack_Anim_Montage.Snake_range_attack_Anim_Montage"
    (:OnCompleted
      _)
    (:OnInterrupted
      _))
  (Variables|Default|SetAttacking false)
  (Default|CallOnAttackEnd))

(fn ConstructionScript
  (|CallParentFunction))